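; Player-controlled eight-legged spider with procedural foot placement; axis inputs move, turn and raise the body, with raising also updating ClimberComponent's body height.
; Each tick, every foot socket is projected onto its last ground plane and compared against FootRange.
; Out-of-range feet line-trace along the body's up axis and pass the hit location to that leg's ABP_Spider effector.
; A sine counter adds body bob and yaw sway.
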(event EventTick
  (params (DeltaSeconds :type Float%20%28single-precision%29))
  ;[1 0.8453 0.04879 0.296] Actual Stuff
  (CallFunction|FixLegs)
  ;[0.5097 1 0.03538 0.45] Idle Up | Down motion
  (CallFunction|MoveBody))

(event Input|AxisEvents|InputAxisSpideyForward
  (params (AxisValue :type Float%20%28single-precision%29))
  ;[0 0.2732 1 0.392] Control Forward, Backward movements
  (Transformation|AddLocalOffset (Variables|Default|GetSpiderBody) (Math|Vector|MakeVector 0.0 (* AxisValue (Utilities|Time|GetWorldDeltaSeconds) (Variables|Default|GetForwardSpeed)) 0.0) true false))

(event Input|AxisEvents|InputAxisSpideyRight
  (params (AxisValue :type Float%20%28single-precision%29))
  ;[0.3488 0 1 0.471] Control the sideways movements
  (Transformation|AddLocalOffset (Variables|Default|GetSpiderBody) (Math|Vector|MakeVector (* AxisValue (Utilities|Time|GetWorldDeltaSeconds) (Variables|Default|GetForwardSpeed) -1.0) 0.0 0.0) true false))

(event Input|AxisEvents|InputAxisSpideyTurn
  (params (AxisValue :type Float%20%28single-precision%29))
  ;[0.883 0 1 0.495] Control Turnings
  (Transformation|AddLocalRotation (Variables|Default|GetSpiderBody) (Math|Rotator|MakeRotator 0.0 0.0 (* AxisValue (Utilities|Time|GetWorldDeltaSeconds) (Variables|Default|GetTurnSpeed))) false false))

(event Input|AxisEvents|InputAxisSpideyRaise
  (params (AxisValue :type Float%20%28single-precision%29))
  (bind _climbercomponent (Variables|Default|GetClimberComponent))
  ;[1 0 0.3287 0.546] Lift Spider Up or down
  (Transformation|AddLocalOffset (Variables|Default|GetSpiderBody) (Math|Vector|MakeVector 0.0 0.0 (* AxisValue (Utilities|Time|GetWorldDeltaSeconds) (Variables|Default|GetRaiseUpSpeed))) true false)
  (if (!= AxisValue 0.0)
    (Variables|/Game/spider/Spider/BP_WallClimberComponent.BP_WallClimberComponent_C|SetBodyHeight _climbercomponent (Variables|/Game/spider/Spider/BP_WallClimberComponent.BP_WallClimberComponent_C|GetCurrentBodyHeight _climbercomponent))))

(fn ConstructionScript
  (Variables|Default|SetLegs (Utilities|Array|MakeArray (Variables|Default|GetSpiderLeg1) (Variables|Default|GetSpiderLeg2) (Variables|Default|GetSpiderLeg3) (Variables|Default|GetSpiderLeg4) (Variables|Default|GetSpiderLeg5) (Variables|Default|GetSpiderLeg6) (Variables|Default|GetSpiderLeg7) (Variables|Default|GetSpiderLeg8)))
  (Variables|Default|SetFoot%20Locations (Utilities|Array|MakeArray "0, 0, 0" "0, 0, 0" "0, 0, 0" "0, 0, 0" "0, 0, 0" "0, 0, 0" "0, 0, 0" "0, 0, 0"))
  (Variables|Default|SetFootNormals (Utilities|Array|MakeArray "0, 0, 0" "0, 0, 0" "0, 0, 0" "0, 0, 0" "0, 0, 0" "0, 0, 0" "0, 0, 0" "0, 0, 0")))

(fn FixLegs
  (for (_array_element _array_index) (Variables|Default|GetLegs)
    (CallFunction|FixLeg _array_element _array_index)))

(fn FixLeg
  (params (Leg :type Skeletal%20Mesh%20Component%20Object%20Reference) (index :type Integer))
  (bind _spiderbody (Variables|Default|GetSpiderBody))
  (bind _returnvalue (Math|Vector|GetUpVector _spiderbody))
  ;[1 0 0.6519 0.258] Checking is a foot update is needed of not
  (if (CallFunction|NeedFootUpdate Leg index)
    (LocalVariables|Seti index)
    ;[0.3832 0.1852 1 0.475] Drawing Line Trace vertically through the Tip of leg to find ground!
    (LocalVariables|SetSelectedLeg Leg)
    (bind _outhit (Collision|LineTraceByChannel (+ (Transformation|GetSocketLocation (LocalVariables|GetSelectedLeg) "footPosition") (* _returnvalue (Variables|Default|GetLineTrace%20Length))) (+ (Transformation|GetSocketLocation (LocalVariables|GetSelectedLeg) "footPosition") (* _returnvalue (* -1 (Variables|Default|GetLineTrace%20Length)))) "TraceTypeQuery1" false 0 "None"))
    ;[0 0.3948 1 0.554] Next Foot location will be at ground below `footPosition` Socket (Check spider_leg_skeleton).
    (if (.bblockinghit _outhit)
      (Utilities|Array|SetArrayElem (Variables|Default|GetFootNormals) (LocalVariables|Geti) (.normal _outhit))
      (Utilities|Array|SetArrayElem (Variables|Default|GetFoot%20Locations) (LocalVariables|Geti) (.location _outhit))
      (bind _asabp_spider (Utilities|Casting|CastToABP_Spider (Components|SkeletalMesh|GetAnimInstance (LocalVariables|GetSelectedLeg))))
      (Variables|/Game/spider/Spider/ABP_Spider.ABP_Spider_C|SetEffectorTransform _asabp_spider (Math|Transform|MakeTransform (Utilities|Array|Get(acopy) (Variables|Default|GetFoot%20Locations) (LocalVariables|Geti)) "0, 0, 0" "1,1,1"))
      (else
        (Variables|Default|SetInGround (.bblockinghit _outhit))))))

(fn NeedFootUpdate
  (params (Foot :type Skeletal%20Mesh%20Component%20Object%20Reference) (Index :type Integer))
  (bind _foot_locations (Variables|Default|GetFoot%20Locations))
  (bind _output (Utilities|Array|Get(acopy) _foot_locations Index))
  ;[1 0.1805 0 0.255] Check if difference between the horizontal coords of `footPosition` socket and previously assigned location stays within the 'FootRange' value, If it does, then no update is needed.
  (bind _new_foot_location__p2_ (CallFunction|FindFootLocation (Transformation|GetSocketLocation Foot "footPosition") (Utilities|Array|Get(acopy) (Variables|Default|GetFootNormals) Index) _output))
  (return (not (<= (Math|Vector|VectorLength (- _new_foot_location__p2_ _output)) (Variables|Default|GetFootRange)))))

(fn MoveBody
  (Transformation|AddLocalOffset (Variables|Default|GetSpiderBody) (Math|Vector|MakeVector 0.0 0.0 (* (Math|Trig|Sin(Degrees) (Variables|Default|GetSpiderMovementBodyCounter)) (Utilities|Time|GetWorldDeltaSeconds) (Variables|Default|GetSpiderMovementVerticalFactor))) true false)
  (Transformation|AddLocalRotation (Variables|Default|GetSpiderBody) (Math|Rotator|MakeRotator 0.0 0.0 (/ (* (Math|Trig|Sin(Degrees) (Variables|Default|GetSpiderMovementBodyCounter)) (Utilities|Time|GetWorldDeltaSeconds) (Variables|Default|GetSpiderMovementVerticalFactor)) (Variables|Default|GetSpiderMovementHorizontalFactor))) false false)
  (if (> (Variables|Default|GetSpiderMovementBodyCounter) 359.0)
    (Variables|Default|SetSpiderMovementBodyCounter 0.0)
    (else
      (Variables|Default|SetSpiderMovementBodyCounter (+ (Variables|Default|GetSpiderMovementVerticalSpeed) (Variables|Default|GetSpiderMovementBodyCounter))))))

(fn AlignArrow
  (bind _output_get (LocalVariables|SetCurrentLocation (Transformation|GetWorldLocation (Variables|Default|GetSpiderBody))))
  (Transformation|SetWorldRotation (Variables|Default|GetArrow) (Math|Rotator|FindLookatRotation (Variables|Default|GetSpiderLocation) _output_get) false false)
  (Variables|Default|SetSpiderLocation (LocalVariables|GetCurrentLocation)))

(fn FindFootLocation
  (params (footLocation%20%28P3%29 :type Vector%20%28by%20ref%29) (normal%20%28N%29 :type Vector%20%28by%20ref%29) (prev%20footPoint%20%28P1%29 :type Vector%20%28by%20ref%29))
  (return (+ footLocation%20%28P3%29 (* normal%20%28N%29 (CallFunction|FindLamda footLocation%20%28P3%29 normal%20%28N%29 prev%20footPoint%20%28P1%29)))))

(fn FindLamda
  (params (Foot%20Location%20%28P3%29 :type Vector%20%28by%20ref%29) (Normal%20%28N%29 :type Vector%20%28by%20ref%29) (Prev%20Foot%20Point%20%28P1%29 :type Vector%20%28by%20ref%29))
  (return (/ (- (+ (* (.x Normal%20%28N%29) (.x Prev%20Foot%20Point%20%28P1%29)) (* (.y Normal%20%28N%29) (.y Prev%20Foot%20Point%20%28P1%29)) (* (.z Normal%20%28N%29) (.z Prev%20Foot%20Point%20%28P1%29))) (+ (* (.x Foot%20Location%20%28P3%29) (.x Normal%20%28N%29)) (* (.y Foot%20Location%20%28P3%29) (.y Normal%20%28N%29)) (* (.z Foot%20Location%20%28P3%29) (.z Normal%20%28N%29)))) (+ (Math|Float|Square (.x Normal%20%28N%29)) (Math|Float|Square (.y Normal%20%28N%29)) (Math|Float|Square (.z Normal%20%28N%29))))))
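; Actor component that keeps its owner, likely a spider, oriented to and hovering over the surface beneath it for wall climbing.
; Each tick it traces along the owner's local down axis and stores the hit distance as the current body height.
; On a hit, it interpolates pitch and roll toward the surface normal while preserving yaw.
; It then applies a swept local Z offset to restore the target body height.
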(event EventTick
  (params (DeltaSeconds :type Float%20%28single-precision%29))
  (bind _returnvalue (Components|GetOwner))
  (bind _returnvalue_2 (Components|GetOwner))
  (bind _returnvalue_3 (Components|GetOwner))
  (bind _returnvalue_4 (Transformation|GetActorLocation _returnvalue))
  (bind _returnvalue_5 (Transformation|GetActorRotation _returnvalue_2))
  (bind _outhit (Collision|LineTraceByChannel _returnvalue_4 (+ _returnvalue_4 (* (Transformation|GetActorUpVector _returnvalue) -6e+02)) "TraceTypeQuery1" false 0 "None"))
  (if (.bblockinghit _outhit)
    (Variables|Default|SetCurrentBodyHeight (.distance _outhit))
    (Transformation|SetActorRotation _returnvalue_3 (Math|Interpolation|RInterpTo _returnvalue_5 (Math|Rotator|MakeRotator (.Roll (Math|Rotator|BreakRotator (Math|Rotator|MakeRotfromZX (.normal _outhit) (Transformation|GetActorForwardVector _returnvalue_2)))) (.Pitch (Math|Rotator|BreakRotator (Math|Rotator|MakeRotfromZY (.normal _outhit) (Transformation|GetActorRightVector _returnvalue_2)))) (.Yaw (Math|Rotator|BreakRotator _returnvalue_5))) (Utilities|Time|GetWorldDeltaSeconds) 1e+01))
    (Transformation|AddActorLocalOffset _returnvalue_3 (Math|Vector|MakeVector 0.0 0.0 (- (Variables|Default|GetBodyHeight) (.distance _outhit))) true true)))
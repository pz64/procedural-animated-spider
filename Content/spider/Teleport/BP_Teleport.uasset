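; Teleporter actor that moves any actor overlapping it to the transform of its FinalLocation target actor, including rotation and scale.
; On BeginPlay it applies the configured label and color to its TeleportText, or prints a warning if no target is set.
; Each tick it turns the text to face the first player's pawn.
; The overlap handler does not check that the target is valid.
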(event EventBeginPlay
  (bind _teleport_text (Variables|Default|GetTeleport%20Text))
  (Utilities|IsValid (Variables|Modify|GetFinalLocation)
    (:Is%20Valid
      (Rendering|Components|TextRender|SetText _teleport_text (Utilities|Text|ToText(String) (Variables|Modify|GetText)))
      (Rendering|Components|TextRender|SetTextRenderColor _teleport_text (Variables|Modify|GetColor)))
    (:Is%20Not%20Valid
      (Development|PrintString "Target not set" true true "(R=1.000000,G=0.191731,B=0.000000,A=1.000000)"))))

(event Collision|EventActorBeginOverlap
  (params (OtherActor :type Actor%20Object%20Reference))
  (Transformation|SetActorTransform OtherActor (Transformation|GetActorTransform (Variables|Modify|GetFinalLocation))))

(event EventTick
  (params (DeltaSeconds :type Float%20%28single-precision%29))
  (Transformation|SetWorldRotation (Variables|Default|GetTeleport%20Text) (Math|Rotator|MakeRotfromX (- (Transformation|GetActorLocation (Game|Player|GetPlayerPawn 0)) (Transformation|GetActorLocation))) false false))

(fn ConstructionScript)
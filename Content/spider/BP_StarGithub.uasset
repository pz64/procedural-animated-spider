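; BP_StarGithub is an actor that displays a scripted promotional message for the project's GitHub release through a text render component.
; On BeginPlay, a single linear chain of Delay nodes steps through hard-coded lines, setting each on the TextRender.
; The lines announce the GitHub push, point to a bio link, ask for stars and pull requests, then sign off with thanks.
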(event EventBeginPlay
  (Utilities|FlowControl|Delay 5.0)
  (bind _output_get (Variables|Default|SetText "Hi"))
  (Rendering|Components|TextRender|SetText (Variables|Default|GetTextRender) _output_get)
  (Utilities|FlowControl|Delay 2.0)
  (bind _output_get_2 (Variables|Default|SetText "I've pushed this project in Github! "))
  (Rendering|Components|TextRender|SetText (Variables|Default|GetTextRender) _output_get_2)
  (Utilities|FlowControl|Delay 2.0)
  (bind _output_get_3 (Variables|Default|SetText "Link in the BIO!"))
  (Rendering|Components|TextRender|SetText (Variables|Default|GetTextRender) _output_get_3)
  (Utilities|FlowControl|Delay 2.0)
  (bind _output_get_4 (Variables|Default|SetText "Link in the BIO!"))
  (Rendering|Components|TextRender|SetText (Variables|Default|GetTextRender) _output_get_4)
  (Utilities|FlowControl|Delay 3.0)
  (bind _output_get_5 (Variables|Default|SetText "Give Star to support this Project. Also expecting pull requests!.."))
  (Rendering|Components|TextRender|SetText (Variables|Default|GetTextRender) _output_get_5)
  (Utilities|FlowControl|Delay 6.0)
  (bind _output_get_6 (Variables|Default|SetText "..."))
  (Rendering|Components|TextRender|SetText (Variables|Default|GetTextRender) _output_get_6)
  (Utilities|FlowControl|Delay 2.0)
  (bind _output_get_7 (Variables|Default|SetText "Lots of glitches tho  :)  !!!"))
  (Rendering|Components|TextRender|SetText (Variables|Default|GetTextRender) _output_get_7)
  (Utilities|FlowControl|Delay 0.7)
  (bind _output_get_8 (Variables|Default|SetText "Thank You!!"))
  (Rendering|Components|TextRender|SetText (Variables|Default|GetTextRender) _output_get_8))

(fn ConstructionScript)